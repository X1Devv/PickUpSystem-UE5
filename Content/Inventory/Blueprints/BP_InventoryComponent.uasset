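; Inventory component that holds a fixed number of item slots, created empty and indexed on BeginPlay.
; AddItem finds the first empty slot, looks up the item ID in DT_ItemData and fills the slot with that row, adding the amount to its CurrentQuantity.
; A successful add fires OnItemAdded with the slot data and returns true.
; Items always take an empty slot, with no stacking onto occupied ones.
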(event `self.ReceiveBeginPlay`
  (`self.InitSlot`))

(fn `AddItem`
  (params (ItemID :type String) (Amount :type Integer))
  (returns (`Success?` :type Boolean))
  (`KismetSystemLibrary.PrintString` (`KismetStringLibrary.Concat_StrStr` "Item " ItemID " added | amount: " (`KismetStringLibrary.Conv_IntToString` Amount)) true true (struct :`G` 0.66 :`B` 1.0 :`A` 1.0) 5.0)
  (bind (_emptyslotavalible _index) (`self.CheckEmptySlot`))
  (if _emptyslotavalible
    (bind _returnvalue (`|GetDataTableRow` "/Game/Inventory/Blueprints/DT_ItemData.DT_ItemData" (`KismetStringLibrary.Conv_StringToName` (`local.ItemID`)))
      (:`then`
        (bind _structout (setmembers `/Game/Inventory/Blueprints/S_Item` :`StructRef` _returnvalue :`CurrentQuantity` (+ (`local.Amount`) (`.CurrentQuantity_29_B8F3A3C34AD7D755F0B9C482F16EECE6` (break `/Game/Inventory/Blueprints/S_Item` _returnvalue)))))
        (bind _structout_2 (setmembers `/Game/Inventory/Blueprints/S_InventorySlotData` :`StructRef` (`|GetArrayItem` (`self.InventorySlots`) _index) :`IsEmpty` false :`ItemData` _structout))
        (`self.OnItemAdded` _structout_2)
        (return true)))))

(fn `CheckEmptySlot`
  (returns (EmptySlotAvalible :type Boolean) (Index :type Integer))
  (for (_array_element _array_index) (`self.InventorySlots`)
    (if (`.IsEmpty_1_0CCAEE50477A4A31D472B6AF1C886EDB` (break `/Game/Inventory/Blueprints/S_InventorySlotData` _array_element))
      (`|ExecutionSequence`
        (:`then_0`
          (break))
        (:`then_1`
          (return true _array_index)))))
  (return false -1))

(fn `InitSlot`
  (for _index (range (`self.NumSlot`))
    (`KismetArrayLibrary.Array_Add` (`self.InventorySlots`) (make `/Game/Inventory/Blueprints/S_InventorySlotData` true (struct :`ItemGroup` "NewEnumerator0") _index))))